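; Demo actor that exercises struct reflection helpers on a test struct, FRTTestStruct.
; BeginPlay calls the parent, then initializes the struct with empty defaults.
; The GetPPS event parses it into a custom Property Parser Struct (PPS).
; Unconnected nodes show further helpers for setting struct values from a TMap, reading property maps, and querying PPS key-values and children, but none of them run.
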(event Custom|GetPPS
  ;[1 1 1] 将结构体解析为 PPS(自定义的结构体)
  (Variables|Default|SetOut%20Property%20Parser%20Struct (Class|ReflectionToolLib|GetPropertyParserStruct (Variables|Default|GetF%20RT%20Test%20Struct))))

(event EventBeginPlay
  (|CallParentFunction)
  (Variables|Default|SetF%20RT%20Test%20Struct (Utilities|Struct|MakeF_RT_TestStruct false 0.0)))

(fn ConstructionScript)